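; BP_Floor is a floor segment that drives score and continued floor generation as the chicken passes through it.
; On BeginPlay it has a random chance to spawn a BP_Coin at one of three coin spawn points.
; When a BP_Chicken first overlaps TriggerZone, it increments the score through the chicken's GameManager and tells FloorSpawner to spawn another floor.
; A Passed flag keeps each segment from triggering again.
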(event OnComponentBeginOverlap(TriggerZone)
  (params (OverlappedComponent :type Primitive%20Component%20Object%20Reference) (OtherActor :type Actor%20Object%20Reference) (OtherComp :type Primitive%20Component%20Object%20Reference) (OtherBodyIndex :type Integer) (bFromSweep :type Boolean) (SweepResult :type Hit%20Result%20Structure%20%28by%20ref%29))
  (bind _asbp_chicken (Utilities|Casting|CastToBP_Chicken OtherActor))
  (if (not (Variables|Default|GetPassed))
    (Default|IncrementScore (Variables|/Game/Chicken_Assets/BP_Chicken.BP_Chicken_C|GetGameManager _asbp_chicken))
    (Default|SpawnFlooratSpawnPoint (Variables|Default|GetFloorSpawner))
    (Variables|Default|SetPassed true)))

(event EventBeginPlay
  (bind _coinspawn0 (Variables|Default|GetCoinSpawn0))
  (bind _coinspawn1 (Variables|Default|GetCoinSpawn1))
  (bind _coinspawn2 (Variables|Default|GetCoinSpawn2))
  (bind _array (Utilities|Array|MakeArray _coinspawn0 _coinspawn1 _coinspawn2))
  (if (<= (Math|Random|RandomInteger 5) 1)
    (Game|SpawnActorfromClass "/Game/Game_World/Pickups/BP_Coin.BP_Coin_C" (Math|Transform|MakeTransform (Transformation|GetWorldLocation (Utilities|Array|Get(acopy) _array (Math|Random|RandomInteger (Utilities|Array|Length _array)))) "0, 0, 0" "1,1,1") "Undefined" 0 0)))

(event Collision|EventActorBeginOverlap
  (params (OtherActor :type Actor%20Object%20Reference)))

(event EventTick
  (params (DeltaSeconds :type Float%20%28single-precision%29)))

(fn ConstructionScript)