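; Game manager for a chicken game that acts as the auto-scrolling camera and tracks score, coins and high score.
; Tick pushes it along +X until the chicken is hit, spawning a single eagle targeting the chicken if its screen projection fails.
; Increment functions update the score widget created on BeginPlay.
; The high score loads from a save slot in the construction script and saves on EndPlay.
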(event EventBeginPlay
  (bind _returnvalue (UserInterface|CreateWidget "/Game/UI/WBP_ScoreTracker.WBP_ScoreTracker_C"))
  (UserInterface|Viewport|AddtoViewport _returnvalue 0)
  (Variables|/Game/UI/WBP_ScoreTracker.WBP_ScoreTracker_C|SetGameManager _returnvalue self)
  (Variables|Default|SetScoreWidget _returnvalue)
  (Variables|Default|SetbFindCameraComponentWhenViewTarget true)
  (Game|Player|SetViewTargetwithBlend (Game|GetPlayerController 0) self 0.0 "VTBlend_Linear" 0.0 false)
  (bind _outactors (Actor|GetAllActorsOfClass "/Game/Chicken_Assets/BP_Chicken.BP_Chicken_C"))
  (Variables|Default|SetPlayer (Utilities|Array|Get(acopy) _outactors))
  (Default|UpdateTopScore (Variables|Default|GetScoreWidget)))

(event Collision|EventActorBeginOverlap
  (params (OtherActor :type Actor%20Object%20Reference)))

(event EventTick
  (params (DeltaSeconds :type Float%20%28single-precision%29))
  (if (not (Variables|/Game/Chicken_Assets/BP_Chicken.BP_Chicken_C|GetHit (Variables|Default|GetPlayer)))
    (Pawn|Input|AddMovementInput "1.000000, 0, 0" 1e+02 false)
    (bind _returnvalue (Class|Pawn|ConsumeMovementInputVector))
    (Transformation|AddActorLocalOffset (* _returnvalue DeltaSeconds) true false)
    (CallFunction|CheckPlayer)))

(event EventEndPlay
  (params (EndPlayReason :type EEndPlayReason%20Enum :default "Destroyed"))
  (bind _savegameinstance (Variables|Default|GetSaveGameInstance))
  (Variables|/Game/BP_SaveHighScore.BP_SaveHighScore_C|SetHighScore _savegameinstance (Variables|Default|GetCurrentHighScore))
  (SaveGame|SaveGametoSlot _savegameinstance (Variables|/Game/BP_SaveHighScore.BP_SaveHighScore_C|GetSaveFileID _savegameinstance))
  (Development|PrintString "Saved game data"))

(fn ConstructionScript
  (bind _returnvalue (SaveGame|CreateSaveGameObject "/Game/BP_SaveHighScore.BP_SaveHighScore_C"))
  (bind _output_get (Variables|Default|SetSaveGameInstance _returnvalue))
  (bind _returnvalue_2 (SaveGame|LoadGamefromSlot (Variables|/Game/BP_SaveHighScore.BP_SaveHighScore_C|GetSaveFileID _output_get)))
  (bind _asbp_save_high_score (Utilities|Casting|CastToBP_SaveHighScore _returnvalue_2))
  (bind _output_get_2 (Variables|Default|SetSaveGameInstance _asbp_save_high_score))
  (Variables|Default|SetCurrentHighScore (Variables|/Game/BP_SaveHighScore.BP_SaveHighScore_C|GetHighScore _output_get_2))
  (Development|PrintString "Loaded game data"))

(fn IncrementScore
  (bind _output_get (Variables|Default|SetScore (+ (Variables|Default|GetScore) 1)))
  (Default|UpdateScoreCounter (Variables|Default|GetScoreWidget))
  (if (> _output_get (Variables|Default|GetCurrentHighScore))
    (Variables|Default|SetCurrentHighScore (Variables|Default|GetScore))
    (Default|UpdateTopScore (Variables|Default|GetScoreWidget))))

(fn CheckPlayer
  (if (not (.ReturnValue (Class|GameplayStatics|ProjectWorldtoScreen (Game|GetPlayerController 0) (Transformation|GetActorLocation (Variables|Default|GetPlayer)) true)))
    (if (not (Variables|Default|GetEagleSent))
      (bind _returnvalue (Game|SpawnActorfromClass "/Game/Game_World/Eagle/BP_Eagle.BP_Eagle_C" (Math|Transform|MakeTransform (Math|Vector|MakeVector (+ (.x (Transformation|GetActorLocation (Variables|Default|GetPlayer))) 8e+02) (.y (Transformation|GetActorLocation (Variables|Default|GetPlayer))) (+ (.z (Transformation|GetActorLocation (Variables|Default|GetPlayer))) 1e+02)) "0, 0, 0" "1,1,1") "Undefined" 0 0))
      (Variables|/Game/Game_World/Eagle/BP_Eagle.BP_Eagle_C|SetPlayer _returnvalue (Variables|Default|GetPlayer))
      (Variables|Default|SetEagleSent true))))

(fn IncrementCoins
  (Math|Integer|IncrementInt (Variables|Default|GetCoinsCollected)
    (:%20%20
      (Default|UpdateCoinCounter (Variables|Default|GetScoreWidget)))))