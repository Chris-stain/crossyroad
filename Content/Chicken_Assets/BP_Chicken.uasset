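; Player character for a hop-style road-crossing game, moving in fixed swept steps with a jump on WASD key release.
; Construction finds the game manager and picks a random chicken or duck mesh and voice, played on some hops.
; Overlapping coins increments the manager's count and destroys them.
; Tick watches an externally set Hit flag, then disables input and collision, bursts feathers and shows the game-over widget after a short delay.
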(event EventBeginPlay)

(event Collision|EventActorBeginOverlap
  (params (OtherActor :type Actor%20Object%20Reference))
  (bind _asbp_coin (Utilities|Casting|CastToBP_Coin OtherActor))
  (Default|IncrementCoins (Variables|Default|GetGameManager))
  (Actor|DestroyActor _asbp_coin)
  (Audio|Components|Audio|Play (Variables|Default|GetCoinAudio) 0.0))

(event EventTick
  (params (DeltaSeconds :type Float%20%28single-precision%29))
  (if (and (Variables|Default|GetHit) (not (Variables|Default|GetGameEnd)))
    (Input|DisableInput 0)
    (Collision|SetActorEnableCollision false)
    (Physics|SetEnableGravity (Variables|Default|GetStaticMesh) false)
    (CallFunction|CreateFeathers)
    (Utilities|FlowControl|Delay 0.5)
    (CallFunction|DisplayGameOver)
    (Variables|/Script/Engine.PlayerController|SetbShowMouseCursor (Game|GetPlayerController 0) true)
    (Variables|Default|SetGameEnd true)))

(event Input|ActionEvents|InputActionMove_X
  (params (Key :type Key%20Structure))
  (:Released
    (if (== Key "W")
      (CallFunction|MoveForward)
      (CallFunction|RandomMoveSound)
      (else
        (CallFunction|MoveBackward)
        (CallFunction|RandomMoveSound)))))

(event Input|ActionEvents|InputActionMove_Y
  (params (Key :type Key%20Structure))
  (:Released
    (if (== Key "A")
      (CallFunction|MoveLeft)
      (CallFunction|RandomMoveSound)
      (else
        (CallFunction|MoveRight)
        (CallFunction|RandomMoveSound)))))

(fn ConstructionScript
  (bind _outactors (Actor|GetAllActorsOfClass "/Game/BP_GameManager.BP_GameManager_C"))
  (Variables|Default|SetGameManager (Utilities|Array|Get(acopy) _outactors))
  (Variables|/Script/Engine.CharacterMovementComponent|SetbOrientRotationToMovement (Variables|Character|GetCharacterMovement) true)
  (CallFunction|SetRandomMesh))

(fn DisplayGameOver
  (bind _returnvalue (UserInterface|CreateWidget "/Game/UI/WBP_GameOverWidget.WBP_GameOverWidget_C"))
  (UserInterface|Viewport|AddtoViewport _returnvalue 0))

(fn MoveBackward
  (Character|Jump)
  (Transformation|SetActorLocationAndRotation (+ (Transformation|GetActorLocation) (* (Transformation|GetActorForwardVector) -2e+02)) (Math|Rotator|MakeRotator 0.0 0.0 -1.0) true))

(fn MoveForward
  (Character|Jump)
  (Transformation|SetActorLocationAndRotation (+ (Transformation|GetActorLocation) (* (Transformation|GetActorForwardVector) 2e+02)) (Math|Rotator|MakeRotator 0.0 0.0 1.0) true))

(fn MoveRight
  (Character|Jump)
  (Transformation|SetActorLocationAndRotation (+ (Transformation|GetActorLocation) (* (Transformation|GetActorRightVector) 2e+02)) (Math|Rotator|MakeRotator 0.0 0.0 -0.5) true))

(fn MoveLeft
  (Character|Jump)
  (Transformation|SetActorLocationAndRotation (+ (Transformation|GetActorLocation) (* (Transformation|GetActorRightVector) -2e+02)) (Math|Rotator|MakeRotator 0.0 0.0 0.5) true))

(fn CreateFeathers
  (Effects|SpawnEmitteratLocation (Variables|Default|GetFeathers) (Transformation|GetActorLocation self)))

(fn SetRandomMesh
  (bind _staticmesh (Variables|Default|GetStaticMesh))
  (bind _moveaudio (Variables|Default|GetMoveAudio))
  (switch int (Math|Random|RandomInteger 4)
    (:0
      (Components|StaticMesh|SetStaticMesh _staticmesh "/Game/Chicken_Assets/cross_road_chicken.cross_road_chicken")
      (Audio|Components|Audio|SetSound _moveaudio "/Game/Audio/PLayer/buck1.buck1"))
    (:1
      (Components|StaticMesh|SetStaticMesh _staticmesh "/Game/Chicken_Assets/cross_road_duck.cross_road_duck")
      (Audio|Components|Audio|SetSound _moveaudio "/Game/Audio/PLayer/quack3.quack3"))
    (:2
      (Components|StaticMesh|SetStaticMesh _staticmesh "/Game/Chicken_Assets/cross_road_chicken.cross_road_chicken")
      (Audio|Components|Audio|SetSound _moveaudio "/Game/Audio/PLayer/frog1.frog1"))
    (:3
      (Components|StaticMesh|SetStaticMesh _staticmesh "/Game/Chicken_Assets/cross_road_chicken.cross_road_chicken")
      (Audio|Components|Audio|SetSound _moveaudio "/Game/Audio/PLayer/sheep1.sheep1"))))

(fn RandomMoveSound
  (Audio|Components|Audio|Play (Variables|Default|GetJumpAudio) 0.0)
  (if (<= (Math|Random|RandomInteger 10) 4)
    (Audio|Components|Audio|Play (Variables|Default|GetMoveAudio) 0.0)))